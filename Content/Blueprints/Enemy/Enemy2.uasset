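; Enemy2 is an enemy actor that damages the player on contact and is destroyed by projectiles.
; Its Box overlap handler reduces an unshielded PlayerCharacter's health and briefly prints the new value on screen.
; A Projectile overlap destroys both the enemy and the projectile, reports the kill to the player character through EnemyKills, and spawns an explosion effect and sound.
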(event `self.Box.OnComponentBeginOverlap`
  (params (OverlappedComponent :type "PrimitiveComponent Object Reference") (OtherActor :type "Actor Object Reference") (OtherComp :type "PrimitiveComponent Object Reference") (OtherBodyIndex :type Integer) (bFromSweep :type Boolean) (SweepResult :type "HitResult Structure (by ref)"))
  (bind _returnvalue (`self.K2_GetActorLocation`))
  ;[1 1 1] Decrease player health on enemy touch.
  (`|ExecutionSequence`
    (:`then_0`
      (bind _asplayer_character (cast `/Game/Blueprints/Player/PlayerCharacter` OtherActor))
      (if (not (`/Game/Blueprints/Player/PlayerCharacter.isShielded` _asplayer_character))
        (bind _output_get (set `/Game/Blueprints/Player/PlayerCharacter.playerHealth` (- (`/Game/Blueprints/Player/PlayerCharacter.playerHealth` _asplayer_character) 10) _asplayer_character))
        (`KismetSystemLibrary.PrintString` (`KismetStringLibrary.Conv_IntToString` _output_get) true false (struct :`R` 0.53125 :`G` 0.029807 :`A` 1.0) 1.0)))
    (:`then_1`
      (bind _asprojectile (cast `/Game/Blueprints/Player/Projectile` OtherActor))
      (`self.K2_DestroyActor`)
      (bind _asplayer_character_2 (cast `/Game/Blueprints/Player/PlayerCharacter` (`GameplayStatics.GetPlayerCharacter` 0)))
      (`/Game/Blueprints/Player/PlayerCharacter.EnemyKills` _asplayer_character_2 (`/Game/Blueprints/Player/PlayerCharacter.enemyDestroyed` _asplayer_character_2))
      (`GameplayStatics.SpawnEmitterAtLocation` "/Game/StarterContent/Particles/P_Explosion.P_Explosion" _returnvalue) ; Enemy Explosion On Destruction
      (`GameplayStatics.SpawnSoundAtLocation` "/Game/Audio/ENEMYEXPLOSION__ByLiamGsfx__SFX.ENEMYEXPLOSION__ByLiamGsfx__SFX" _returnvalue (struct) 0.35) ; Explosion Sound Settings
      (`self.K2_DestroyActor` _asprojectile))))

(fn `UserConstructionScript`)