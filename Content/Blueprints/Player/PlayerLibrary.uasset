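; PlayerLibrary holds shared functions for damaging the player and handling death.
; TakeDamage casts player 0 to PlayerCharacter, has its PlayerHealth1 member compute the new health through PlayerDamaged, and stores the result in PlayerHealth.
; When health drops to zero or below it calls Death, which only prints a debug message.
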(fn `Death`
  (`KismetSystemLibrary.PrintString` null "DIED"))

(fn `TakeDamage`
  (params (Damage :type Integer))
  (bind _asplayer_character (cast `/Game/Blueprints/Player/PlayerCharacter` (`GameplayStatics.GetPlayerCharacter` null)))
  (bind _newplayerhealth (`/Game/Blueprints/Player/PlayerHealth.PlayerDamaged` (`/Game/Blueprints/Player/PlayerCharacter.PlayerHealth1` _asplayer_character) Damage (`/Game/Blueprints/Player/PlayerCharacter.playerHealth` _asplayer_character)))
  (bind _output_get (set `/Game/Blueprints/Player/PlayerCharacter.playerHealth` _newplayerhealth _asplayer_character))
  (if (<= _output_get 0)
    (`self.Death` null)))