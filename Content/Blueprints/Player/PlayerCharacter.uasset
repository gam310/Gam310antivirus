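; Player character with world-axis movement, a once-per-second data counter and timed speed boosts.
; Tick drives the counter, throttled by a Delay and printed on screen, and a health check that opens Level01 when PlayerHealth drops below 1.
; Overlapping a Speed_Booster while unboosted destroys the pickup and raises walk speed for ten seconds; IsBoosted is set but never cleared here.
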(event `self.ReceiveTick`
  (params (DeltaSeconds :type "Float (single-precision)"))
  ;[1 1 1] Event Ticks
  (`self.DataTick` 0.0)
  (`self.DestroyTick` 0.0))

(event `DataTick`
  (params (`Delta Seconds` :type "Float (double-precision)"))
  ;[1 1 1] Player Data
  (`KismetSystemLibrary.Delay` 1.0)
  (bind _output_get (set `self.dataCollected` (+ (`self.dataCollected`) 1)))
  (`KismetSystemLibrary.PrintString` (`KismetStringLibrary.Conv_IntToString` _output_get) true false (struct :`R` 0.078022 :`G` 1.0 :`B` 0.109892 :`A` 1.0) 1.0))

(event `DestroyTick`
  (params (`Delta Seconds` :type "Float (double-precision)"))
  ;[1 1 1] Player Destroyed. Restart Level?
  (bind _output_get (set `self.isDestroyed` (< (`self.playerHealth`) 1)))
  (if _output_get
    (`GameplayStatics.OpenLevel` (`self.Level01`))))

(event `InputAxis|UpOrDown`
  (params (AxisValue :type "Float (single-precision)"))
  ;[1 1 1] Player Controls
  (`self.AddMovementInput` (1.0 0.0 0.0) AxisValue))

(event `InputAxis|LeftorRight`
  (params (AxisValue :type "Float (single-precision)"))
  ;[1 1 1] Player Controls
  (`self.AddMovementInput` (0.0 1.0 0.0) AxisValue))

(event `self.ReceiveActorBeginOverlap`
  (params (OtherActor :type "Actor Object Reference"))
  (bind _charactermovement (`self.CharacterMovement`))
  ;[1 1 1] Speed Boost
  (bind _asspeed_booster (cast `/Game/Blueprints/Speed_Booster` OtherActor))
  (if (<= (`KismetMathLibrary.FTrunc` (`CharacterMovementComponent.MaxWalkSpeed` (`self.CharacterMovement`))) 600)
    (`self.K2_DestroyActor` _asspeed_booster)
    (set `self.isBoosted` true)
    (set `CharacterMovementComponent.MaxWalkSpeed` 1000.0 _charactermovement)
    (`KismetSystemLibrary.PrintString` "SPEED INCREASED")
    (`KismetSystemLibrary.Delay` 10.0) ; How long speed boost lasts in secs
    (set `CharacterMovementComponent.MaxWalkSpeed` 600.0 _charactermovement)))

(fn `UserConstructionScript`)